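; Player character Blueprint for distance matching that records where movement starts and where it will stop.
; Axis inputs drive camera look and control-yaw-relative movement, with a correction for diagonal gamepad values.
; Tick derives a Stopped state from move input and, once per transition, saves the start location or predicts the stop location from velocity, friction and braking deceleration.
; Both points are drawn as debug spheres.
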(event `self.ReceiveTick`
  (params (DeltaSeconds :type "Float (single-precision)"))
  (bind _charactermovement (`self.CharacterMovement`))
  (`|ExecutionSequence`
    (:`then_0`
      (if (or (!= (`self.GetInputAxisValue`) 0.0) (!= (`self.GetInputAxisValue`) 0.0))
        (set `self.Stopped` false)
        (`/Engine/EditorBlueprintResources/StandardMacros.DoOnce` false
          (:`Completed`
            (set `self.HasMoved` true)))
        (elif (`self.HasMoved`)
          (set `self.Stopped` true)
          (else
            (set `self.Stopped` false)))))
    (:`then_1`
      (`|ExecutionSequence`
        (:`then_0`
          (if (`self.Stopped`)
            (`/Engine/EditorBlueprintResources/StandardMacros.DoOnce` false :!label _label
              (:`Completed`
                (bind _outstoplocation (`DistanceMatchingPluginBPLibrary.PredictStopLocation` (`self.K2_GetActorLocation`) (`self.GetVelocity`) (`CharacterMovementComponent.GetCurrentAcceleration` _charactermovement) (`CharacterMovementComponent.BrakingFriction` _charactermovement) (`CharacterMovementComponent.BrakingDecelerationWalking` _charactermovement) (`GameplayStatics.GetWorldDeltaSeconds`) 100))
                (bind _output_get (set `self.Stop Location` _outstoplocation))
                (`KismetSystemLibrary.DrawDebugSphere` _output_get 30.0 12 (struct :`R` 0.196295 :`G` 1.0 :`B` 0.432402 :`A` 1.0) 2.0)))
            (else
              (goto _label :!via `Reset`))))
        (:`then_1`
          (if (and (not (`self.Stopped`)) (`self.HasMoved`))
            (`/Engine/EditorBlueprintResources/StandardMacros.DoOnce` false :!label _label_2
              (:`Completed`
                (bind _output_get_2 (set `self.StartLocation` (`self.K2_GetActorLocation`)))
                (`KismetSystemLibrary.DrawDebugSphere` _output_get_2 30.0 12 (struct :`R` 1.0 :`G` 0.153805 :`B` 0.305898 :`A` 1.0) 2.0)))
            (else
              (goto _label_2 :!via `Reset`))))))))

(event `InputAxis|MoveRight`
  (params (AxisValue :type "Float (single-precision)"))
  (`self.PlayerMovementInput` false))

(event `InputAxis|MoveForward`
  (params (AxisValue :type "Float (single-precision)"))
  (`self.PlayerMovementInput` true)
  (set `self.FWD` (> AxisValue 0.0)))

(event `InputAxis|Turn`
  (params (AxisValue :type "Float (single-precision)"))
  (`self.AddControllerYawInput` AxisValue))

(event `InputAxis|LookUp`
  (params (AxisValue :type "Float (single-precision)"))
  (`self.AddControllerPitchInput` AxisValue))

(fn `FixDiagonalGamepadValues`
  (params (`X In` :type "Float (double-precision)") (`Y In` :type "Float (double-precision)"))
  (returns (`X Out` :type "Float (double-precision)") (`Y Out` :type "Float (double-precision)"))
  (return (`KismetMathLibrary.FClamp` (* (`local.X In`) (`KismetMathLibrary.MapRangeClamped` (`KismetMathLibrary.Abs` (`local.Y In`)) 0.0 0.6 1.0 1.2)) -1.0) (`KismetMathLibrary.FClamp` (* (`local.Y In`) (`KismetMathLibrary.MapRangeClamped` (`KismetMathLibrary.Abs` (`local.X In`)) 0.0 0.6 1.0 1.2)) -1.0)))

(fn `GetControllForward/RightVector`
  (returns (ForwardVector :type "Vector Structure") (RightVector :type "Vector Structure"))
  (bind (_returnvalue_roll _returnvalue_pitch _returnvalue_yaw) (`KismetMathLibrary.BreakRotator` (`self.GetControlRotation`)))
  (return (`KismetMathLibrary.GetForwardVector` (`KismetMathLibrary.MakeRotator` 0.0 0.0 _returnvalue_yaw)) (`KismetMathLibrary.GetRightVector` (`KismetMathLibrary.MakeRotator` 0.0 0.0 _returnvalue_yaw))))

(fn `PlayerMovementInput`
  (params (IsMoveForward :type Boolean))
  (bind (_forwardvector _rightvector) (`self.GetControllForward/RightVector`))
  (bind (_x_out _y_out) (`self.FixDiagonalGamepadValues` (`self.GetInputAxisValue`) (`self.GetInputAxisValue`)))
  (if IsMoveForward
    (`self.AddMovementInput` _forwardvector _y_out)
    (else
      (`self.AddMovementInput` _rightvector _x_out))))

(fn `UserConstructionScript`)