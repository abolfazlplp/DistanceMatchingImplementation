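; Player character Blueprint in the DistanceMatching folder that handles movement and look input.
; Turn and LookUp axes feed controller yaw and pitch, while MoveForward and MoveRight call a shared PlayerMovementInput function.
; Movement directions come from control rotation yaw only, so travel follows the view heading on a flat plane.
; FixDiagonalGamepadValues boosts each axis as the other deflects, then clamps it, compensating for weaker diagonal stick input.
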(event `InputAxis|MoveRight`
  (params (AxisValue :type "Float (single-precision)"))
  (`self.PlayerMovementInput` false))

(event `InputAxis|MoveForward`
  (params (AxisValue :type "Float (single-precision)"))
  (`self.PlayerMovementInput` true))

(event `InputAxis|Turn`
  (params (AxisValue :type "Float (single-precision)"))
  (`self.AddControllerYawInput` AxisValue))

(event `InputAxis|LookUp`
  (params (AxisValue :type "Float (single-precision)"))
  (`self.AddControllerPitchInput` AxisValue))

(fn `FixDiagonalGamepadValues`
  (params (`X In` :type "Float (double-precision)") (`Y In` :type "Float (double-precision)"))
  (returns (`X Out` :type "Float (double-precision)") (`Y Out` :type "Float (double-precision)"))
  (return (`KismetMathLibrary.FClamp` (* (`local.X In`) (`KismetMathLibrary.MapRangeClamped` (`KismetMathLibrary.Abs` (`local.Y In`)) 0.0 0.6 1.0 1.2)) -1.0) (`KismetMathLibrary.FClamp` (* (`local.Y In`) (`KismetMathLibrary.MapRangeClamped` (`KismetMathLibrary.Abs` (`local.X In`)) 0.0 0.6 1.0 1.2)) -1.0)))

(fn `GetControllForward/RightVector`
  (returns (ForwardVector :type "Vector Structure") (RightVector :type "Vector Structure"))
  (bind (_returnvalue_roll _returnvalue_pitch _returnvalue_yaw) (`KismetMathLibrary.BreakRotator` (`self.GetControlRotation`)))
  (return (`KismetMathLibrary.GetForwardVector` (`KismetMathLibrary.MakeRotator` 0.0 0.0 _returnvalue_yaw)) (`KismetMathLibrary.GetRightVector` (`KismetMathLibrary.MakeRotator` 0.0 0.0 _returnvalue_yaw))))

(fn `PlayerMovementInput`
  (params (IsMoveForward :type Boolean))
  (bind (_forwardvector _rightvector) (`self.GetControllForward/RightVector`))
  (bind (_x_out _y_out) (`self.FixDiagonalGamepadValues` (`self.GetInputAxisValue`) (`self.GetInputAxisValue`)))
  (if IsMoveForward
    (`self.AddMovementInput` _forwardvector _y_out)
    (else
      (`self.AddMovementInput` _rightvector _x_out))))

(fn `UserConstructionScript`)